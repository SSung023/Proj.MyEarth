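; Test glacier Blueprint that reacts to player contact as a pushable object and toggles custom depth rendering, apparently for a post-process effect.
; On box overlap it stores a flattened unit direction from its construction-time position toward the player and sets IsPushed.
; Tick enables custom depth whenever CanMove is false; ending overlap clears CanMove.
; Nothing here moves the glacier or sets CanMove true.
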(event OnComponentBeginOverlap(Boxcollider)
  (params (OverlappedComponent :type Primitive%20Component%20Object%20Reference) (OtherActor :type Actor%20Object%20Reference) (OtherComp :type Primitive%20Component%20Object%20Reference) (OtherBodyIndex :type Integer) (bFromSweep :type Boolean) (SweepResult :type Hit%20Result%20Structure%20%28by%20ref%29))
  (Utilities|FlowControl|DoOnce false :!label _label
    (:Completed
      (bind _asplayer_character (Utilities|Casting|CastToPlayerCharacter OtherActor))
      (CallFunction|SetDirectionVec _asplayer_character)
      (Variables|Default|SetisPushed true)
      (goto _label Reset))))

(event OnComponentEndOverlap(Boxcollider)
  (params (OverlappedComponent :type Primitive%20Component%20Object%20Reference) (OtherActor :type Actor%20Object%20Reference) (OtherComp :type Primitive%20Component%20Object%20Reference) (OtherBodyIndex :type Integer))
  (Variables|Default|SetcanMove false))

(event EventTick
  (params (DeltaSeconds :type Float%20%28single-precision%29))
  (bind _glacier (Variables|Default|GetGlacier))
  (if (Variables|Default|GetcanMove)
    (Rendering|SetRenderCustomDepth _glacier false)
    (else
      (Rendering|SetRenderCustomDepth _glacier true))))

(fn ConstructionScript
  (Variables|Default|SetcurGPos (Transformation|GetActorLocation)))

(fn SetDirectionVec
  (params (player :type Player%20Character%20Object%20Reference))
  (bind _flattenedvector (CallFunction|FlattenVector (Transformation|GetActorLocation player)))
  (bind _flattenedvector_2 (CallFunction|FlattenVector (Variables|Default|GetcurGPos)))
  (Variables|Default|SetdirectionVec (Math|Vector|GetUnitDirection(Vector) _flattenedvector_2 _flattenedvector)))

(fn FlattenVector
  (params (vec :type Vector))
  (bind (_x _y) (Math|Vector|BreakVector vec))
  (return (Math|Vector|MakeVector _x _y 0.0)))