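; BP_Glacier is a pushable ice block that slides along a horizontal axis each time Push is called.
; Four side colliders set an axis-aligned direction and enable pushing, which Tick shows through custom depth rendering.
; A DoOnce-guarded timeline offsets the actor from its stored position without sweeping, then saves the new position and disables pushing.
; A player-relative direction helper exists but is not called here.
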(event OnComponentBeginOverlap(frontcollider)
  (params (OverlappedComponent :type Primitive%20Component%20Object%20Reference) (OtherActor :type Actor%20Object%20Reference) (OtherComp :type Primitive%20Component%20Object%20Reference) (OtherBodyIndex :type Integer) (bFromSweep :type Boolean) (SweepResult :type Hit%20Result%20Structure%20%28by%20ref%29))
  ;[1 1 1] set directionVector by activated trigger
  (Variables|Default|SetdirectionVec "-1.000000, 0, 0")
  (Variables|Default|SetcanBePushed true))

(event OnComponentBeginOverlap(rightcollider)
  (params (OverlappedComponent :type Primitive%20Component%20Object%20Reference) (OtherActor :type Actor%20Object%20Reference) (OtherComp :type Primitive%20Component%20Object%20Reference) (OtherBodyIndex :type Integer) (bFromSweep :type Boolean) (SweepResult :type Hit%20Result%20Structure%20%28by%20ref%29))
  ;[1 1 1] set directionVector by activated trigger
  (Variables|Default|SetdirectionVec "0.000000,-1.000000, 0")
  (Variables|Default|SetcanBePushed true))

(event OnComponentBeginOverlap(leftcollider)
  (params (OverlappedComponent :type Primitive%20Component%20Object%20Reference) (OtherActor :type Actor%20Object%20Reference) (OtherComp :type Primitive%20Component%20Object%20Reference) (OtherBodyIndex :type Integer) (bFromSweep :type Boolean) (SweepResult :type Hit%20Result%20Structure%20%28by%20ref%29))
  ;[1 1 1] set directionVector by activated trigger
  (Variables|Default|SetdirectionVec "0.000000,1.000000, 0")
  (Variables|Default|SetcanBePushed true))

(event OnComponentBeginOverlap(backcollider)
  (params (OverlappedComponent :type Primitive%20Component%20Object%20Reference) (OtherActor :type Actor%20Object%20Reference) (OtherComp :type Primitive%20Component%20Object%20Reference) (OtherBodyIndex :type Integer) (bFromSweep :type Boolean) (SweepResult :type Hit%20Result%20Structure%20%28by%20ref%29))
  ;[1 1 1] set directionVector by activated trigger
  (Variables|Default|SetdirectionVec "1.000000, 0, 0")
  (Variables|Default|SetcanBePushed true))

(event Custom|Push
  ;[1 1 1] Check glacier condition
  (if (Variables|Default|GetcanBePushed)
    (CallFunction|MoveGlacier)))

(event Custom|MoveGlacier
  ;[1 1 1] Move glacier one block
  (Utilities|FlowControl|DoOnce false :!label _label
    (:Completed
      (bind _newpos (Timeline|updateGlacierPos PlayFromStart)
        (:Update
          (Transformation|SetActorLocation (+ (* (Variables|Default|GetdirectionVec) _newpos) (Variables|Default|GetcurGPos)) false false))
        (:Finished
          (Variables|Default|SetcurGPos (Transformation|GetActorLocation))
          (Variables|Default|SetcanBePushed false)
          (goto _label Reset))))))

(event EventTick
  (params (DeltaSeconds :type Float%20%28single-precision%29))
  (bind _glacier (Variables|Default|GetGlacier))
  (if (Variables|Default|GetcanBePushed)
    (Rendering|SetRenderCustomDepth _glacier true)
    (else
      (Rendering|SetRenderCustomDepth _glacier false))))

(fn ConstructionScript
  (Variables|Default|SetcurGPos (Transformation|GetActorLocation))
  (Rendering|SetRenderCustomDepth (Variables|Default|GetGlacier) false))

(fn SetDirectionVec
  (params (player :type Player%20Character%20Object%20Reference))
  (bind _flattenedvector (CallFunction|FlattenVector (Transformation|GetActorLocation player)))
  (bind _flattenedvector_2 (CallFunction|FlattenVector (Variables|Default|GetcurGPos)))
  (Variables|Default|SetdirectionVec (Math|Vector|GetUnitDirection(Vector) _flattenedvector_2 _flattenedvector)))

(fn FlattenVector
  (params (vec :type Vector))
  (bind (_x _y) (Math|Vector|BreakVector vec))
  (return (Math|Vector|MakeVector _x _y 0.0)))